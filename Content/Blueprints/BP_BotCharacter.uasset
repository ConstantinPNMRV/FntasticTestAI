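; BP_BotCharacter is an AI enemy character that is disabled after four hits from first-person projectiles.
; It caches its BP_BotController on BeginPlay and binds to capsule hit events to count BP_FirstPersonProjectile impacts.
; Damage and death are only printed messages; the fourth hit switches off the behavior tree through the controller.
; Re-enabling the tree through SetEnableBehaviorTree resets the hit counter.
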(event `self.ReceiveBeginPlay`
  ;[1 1 1] BeginPlay
  (`self.InitVariables`)
  (`self.BindEvents`))

(fn `BindEvents`
  (add `PrimitiveComponent.OnComponentHit` (`self.CapsuleComponent`) (`|CreateDelegate` :!event `BindOnComponentHit`)))

(fn `BindOnComponentHit`
  (params (HitComponent :type "PrimitiveComponent Object Reference") (OtherActor :type "Actor Object Reference") (OtherComp :type "PrimitiveComponent Object Reference") (NormalImpulse :type "Vector Structure") (Hit :type "HitResult Structure (by ref)"))
  (locals (L_Projectile :type "/Game/Blueprints/BP_FirstPersonProjectile Object Reference") (L_Hit :type "HitResult Structure"))
  (bind _asbp_first_person_projectile (cast `/Game/Blueprints/BP_FirstPersonProjectile` OtherActor))
  (set `local.L_Projectile` _asbp_first_person_projectile)
  (set `local.L_Hit` Hit)
  (bind _result (`/Engine/EditorBlueprintResources/StandardMacros.IncrementInt` (`self.HitCounter`))
    (:`  `
      (if (== _result 4)
        (`KismetSystemLibrary.PrintString` "Enemy is Dead" true true (struct :`G` 0.66 :`B` 1.0 :`A` 1.0) 5.0)
        (`self.SetEnableBehaviorTree` false)
        (elif (< (`self.HitCounter`) 4)
          (`KismetSystemLibrary.PrintString` "-25 hp" true true (struct :`G` 0.66 :`B` 1.0 :`A` 1.0) 5.0))))))

(fn `InitVariables`
  (bind _asbp_bot_controller (cast `/Game/Blueprints/BP_BotController` (`AIBlueprintHelperLibrary.GetAIController` self)))
  (set `self.BotController` _asbp_bot_controller))

(fn `SetEnableBehaviorTree`
  (params (IsOn :type Boolean))
  (locals (L_IsOn :type Boolean))
  (bind _output_get (set `local.L_IsOn` IsOn))
  (`/Game/Blueprints/BP_BotController.SetEnableBehaviorTree` (`self.BotController`) _output_get)
  (if (`local.L_IsOn`)
    (set `self.HitCounter` 0)))

(fn `UserConstructionScript`
  (`parent.UserConstructionScript`))