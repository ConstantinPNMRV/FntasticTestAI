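; AI controller for BP_BotCharacter that runs its behavior tree and turns perception of the first-person player into blackboard state.
; On BeginPlay it sets patrol points ahead of and behind the bot, then stops tree logic until re-enabled.
; Sight and damage share a handler that tracks the player, or marks the stimulus location as noise on failed sensing.
; Hearing, ignored while tracking, stores a randomized-distance point toward the sound.
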(event `self.ReceiveBeginPlay`
  ;[1 1 1] BeginPlay
  (`self.InitVariables`))

(event `self.AIPerception.OnTargetPerceptionUpdated`
  (params (Actor :type "Actor Object Reference") (Stimulus :type "AIStimulus Structure"))
  ;[1 1 1] Определение чувства, на которое среагировал бот
  (bind _asbp_first_person_character (cast `/Game/Blueprints/BP_FirstPersonCharacter` Actor))
  (set `self.PlayerEnemy` _asbp_first_person_character)
  (bind _output_get (set `self.Stimulas` Stimulus))
  (bind _returnvalue (`AIPerceptionSystem.GetSenseClassForStimulus` _output_get))
  (switch `string` (`KismetSystemLibrary.GetClassDisplayName` _returnvalue)
    (:`AISense_Hearing`
      (`self.BotHearingHandler`))
    (:`AISense_Sight`
      (`self.BotVisionHandler`))
    (:`AISense_Damage`
      (`self.BotDamageHandler`))))

(fn `BotDamageHandler`
  (`self.BotVisionHandler`))

(fn `BotHearingHandler`
  (bind (_age _expirationage _strength _stimuluslocation _receiverlocation) (break `AIStimulus` (`self.Stimulas`)))
  (if (not (`self.IsHasPlayer`))
    (`self.SetIsHearNoise` false)
    (if (`.bSuccessfullySensed` (break `AIStimulus` (`self.Stimulas`)))
      (`self.SetIsHearNoise` true)
      (`BlackboardComponent.SetValueAsVector` (`self.BlackboardComp`) "NoiseLocation" (`self.CalculateNoiseLocation` _stimuluslocation _receiverlocation)))))

(fn `BotVisionHandler`
  (`self.SetIsHearNoise` false)
  (set `self.IsHasPlayer` (`.bSuccessfullySensed` (break `AIStimulus` (`self.Stimulas`))))
  (`BlackboardComponent.SetValueAsBool` (`self.BlackboardComp`) "IsHasPlayer" (`self.IsHasPlayer`))
  (if (`self.IsHasPlayer`)
    (`BlackboardComponent.SetValueAsObject` (`self.BlackboardComp`) "Player" (`self.PlayerEnemy`))
    (else
      (`BlackboardComponent.ClearValue` (`self.BlackboardComp`) "Player")
      (`self.SetIsHearNoise` true)
      (`BlackboardComponent.SetValueAsVector` (`self.BlackboardComp`) "NoiseLocation" (`.StimulusLocation` (break `AIStimulus` (`self.Stimulas`)))))))

(fn `CalculateNoiseLocation`
  (params (StimulusLocation :type "Vector Structure (by ref)") (ReceiverLocation :type "Vector Structure (by ref)"))
  (returns (ReturnValue :type "Vector Structure"))
  (locals (L_StimulusLocation :type "Vector Structure") (L_ReceiverLocation :type "Vector Structure"))
  (set `local.L_StimulusLocation` StimulusLocation)
  (bind _output_get (set `local.L_ReceiverLocation` ReceiverLocation))
  (return (+ (`local.L_ReceiverLocation`) (* (`KismetMathLibrary.GetForwardVector` (`KismetMathLibrary.FindLookAtRotation` _output_get (`local.L_StimulusLocation`))) (`KismetMathLibrary.RandomFloatInRange` 1.0 1000.0)))))

(fn `CalculatePatrolLocations`
  (bind _botcharacter (`self.BotCharacter`))
  (bind _botcharacter_2 (`self.BotCharacter`)
    (:`then`
      (`self.SetPatrolLocations` (+ (`self.K2_GetActorLocation` _botcharacter_2) (* (`self.GetActorForwardVector` _botcharacter_2) 2000.0)) (+ (`self.K2_GetActorLocation` _botcharacter) (* (`self.GetActorForwardVector` _botcharacter) -2000.0))))
    (:`else`)))

(fn `InitVariables`
  (bind _returnvalue (`AIBlueprintHelperLibrary.GetBlackboard` null))
  (`self.RunBehaviorTree` "/Game/Blueprints/BT_BotCharacter.BT_BotCharacter")
  (`/Engine/EditorBlueprintResources/StandardMacros.IsValid` _returnvalue
    (:`Is Valid`
      (set `self.BlackboardComp` _returnvalue)
      (bind _asbp_bot_character (cast `/Game/Blueprints/BP_BotCharacter` (`self.K2_GetPawn` self)))
      (set `self.BotCharacter` _asbp_bot_character)
      (`self.CalculatePatrolLocations`)
      (`self.SetEnableBehaviorTree` false))
    (:`Is Not Valid`
      (`KismetSystemLibrary.PrintString` "Blackboard не найден." true true (struct :`R` 1.0 :`G` 0.006821 :`A` 1.0) 10.0))))

(fn `SetEnableBehaviorTree`
  (params (IsOn :type Boolean))
  (bind _braincomponent (`self.BrainComponent`))
  (if IsOn
    (`BrainComponent.StartLogic` _braincomponent)
    (else
      (`BrainComponent.StopLogic` _braincomponent "Stop"))))

(fn `SetIsHearNoise`
  (params (IsOn :type Boolean))
  (`BlackboardComponent.SetValueAsBool` (`self.BlackboardComp`) "IsHearNoise" IsOn))

(fn `SetPatrolLocations`
  (params (ForwardLocation :type "Vector Structure") (BackwardLocation :type "Vector Structure"))
  (locals (L_ForwardLocation :type "Vector Structure") (L_BackwardLocation :type "Vector Structure"))
  (set `local.L_ForwardLocation` ForwardLocation)
  (set `local.L_BackwardLocation` BackwardLocation)
  (`BlackboardComponent.SetValueAsVector` (`self.BlackboardComp`) "ForwardLocation" (`local.L_ForwardLocation`))
  (`BlackboardComponent.SetValueAsVector` (`self.BlackboardComp`) "BackwardLocation" (`local.L_BackwardLocation`)))

(fn `UserConstructionScript`)